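; BP_DoorDistance is a door that shows an exit text while the player is nearby and closes itself when they leave.
; Tick checks the player pawn's distance against a fixed radius, toggling the text while the door is shut.
; OpenTheDoor, not called within this file, plays the OpenDoor sequence if the player is near.
; Leaving range reverses the sequence, with delays holding back the open-state flag changes.
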(event `self.ReceiveTick`
  (params (DeltaSeconds :type "Float (single-precision)"))
  (bind _exittext (`self.ExitText`))
  (`self.CheckDistance`)
  (if (and (not (`self.IsDoorOpened`)) (`self.IsPlayerNear`))
    (`SceneComponent.SetVisibility` _exittext true false)
    (else
      (`SceneComponent.SetVisibility` _exittext false false)
      (if (`self.IsDoorOpened`)
        (if (not (`self.IsPlayerNear`))
          (`MovieSceneSequencePlayer.PlayReverse` (`LevelSequenceActor.SequencePlayer` (`self.OpenDoor`)))
          (`KismetSystemLibrary.Delay` 2.0)
          (set `self.IsDoorOpened` false))))))

(event `CheckDistance`
  (if (<= (`self.GetDistanceTo` (`GameplayStatics.GetPlayerPawn` 0)) 350.0)
    (set `self.IsPlayerNear` true)
    (else
      (set `self.IsPlayerNear` false))))

(event `OpenTheDoor`
  (bind _sequenceplayer (`LevelSequenceActor.SequencePlayer` (`self.OpenDoor`)))
  (if (and (`self.IsPlayerNear`) (not (`self.IsDoorOpened`)))
    (`MovieSceneSequencePlayer.Play` _sequenceplayer)
    (`KismetSystemLibrary.Delay` 2.0)
    (set `self.IsDoorOpened` true)
    (`SceneComponent.SetVisibility` (`self.ExitText`) false false)
    (`MovieSceneSequencePlayer.Pause` _sequenceplayer)))

(fn `UserConstructionScript`)