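; BP_Door is a door that opens once through a level sequence when the player is near.
; An interior box's overlap events set the proximity flag and toggle the exit text's visibility, with no filter on the overlapping actor.
; The OpenTheDoor event checks proximity and the opened flag, plays the sequence, then after a fixed delay marks the door opened and pauses playback.
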(event `self.Box_interior.OnComponentBeginOverlap`
  (params (OverlappedComponent :type "PrimitiveComponent Object Reference") (OtherActor :type "Actor Object Reference") (OtherComp :type "PrimitiveComponent Object Reference") (OtherBodyIndex :type Integer) (bFromSweep :type Boolean) (SweepResult :type "HitResult Structure (by ref)"))
  (set `self.IsPlayerNear` true)
  (`SceneComponent.ToggleVisibility` (`self.ExitText`) false :!label _label))

(event `self.Box_interior.OnComponentEndOverlap`
  (params (OverlappedComponent :type "PrimitiveComponent Object Reference") (OtherActor :type "Actor Object Reference") (OtherComp :type "PrimitiveComponent Object Reference") (OtherBodyIndex :type Integer))
  (set `self.IsPlayerNear` false)
  (goto _label))

(event `OpenTheDoor`
  (bind _sequenceplayer (`LevelSequenceActor.SequencePlayer` (`self.OpenDoor`)))
  (if (and (`self.IsPlayerNear`) (not (`self.IsDoorOpened`)))
    (`MovieSceneSequencePlayer.Play` _sequenceplayer)
    (`KismetSystemLibrary.Delay` 2.0)
    (set `self.IsDoorOpened` true)
    (`MovieSceneSequencePlayer.Pause` _sequenceplayer)))

(fn `UserConstructionScript`)