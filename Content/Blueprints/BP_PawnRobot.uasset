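; Player robot pawn with movement, mouse look and physics-object pickup and throwing.
; Right mouse line-traces along the camera direction and grabs objects under a mass limit with a runtime-added PhysicsHandle, ignoring Pawn collision until released.
; Tick holds the object at its grab distance along control rotation, while the mouse wheel changes trace reach.
; Left click releases it with an impulse along the capsule's forward vector.
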(event `InputAxis|MoveForward`
  (params (AxisValue :type "Float (single-precision)"))
  (`self.AddMovementInput` (`self.GetActorForwardVector`) AxisValue))

(event `InputAxis|Strafe`
  (params (AxisValue :type "Float (single-precision)"))
  (`self.AddMovementInput` (`self.GetActorRightVector`) AxisValue))

(event `InputAxis|MouseX`
  (params (AxisValue :type "Float (single-precision)"))
  (`self.AddControllerYawInput` AxisValue))

(event `InputAxis|MouseY`
  (params (AxisValue :type "Float (single-precision)"))
  (`self.AddControllerPitchInput` AxisValue))

(event `self.ReceiveTick`
  (params (DeltaSeconds :type "Float (single-precision)"))
  (bind _physicshandle (`self.PhysicsHandle`))
  ;[1 1 1] Pick up location
  (if (`self.PhysicsHandleActive`)
    (bind _output_get (set `self.HandleLocation` (+ (+ (`self.K2_GetActorLocation`) (* (`KismetMathLibrary.GetForwardVector` (`self.GetControlRotation`)) (`self.OtherItemLocation`))) (0.0 0.0 50.0))))
    (`/Engine/EditorBlueprintResources/StandardMacros.IsValid` _physicshandle
      (:`Is Valid`
        (`PhysicsHandleComponent.SetTargetLocationAndRotation` _physicshandle _output_get (`self.GetControlRotation`))))))

(event `InputAxisKey|MouseWheelAxis`
  (params (AxisValue :type "Float (single-precision)"))
  ;[1 1 1] Adjust pickup distance
  (set `self.PickUpDistance` (+ (* AxisValue 25.0) (`self.PickUpDistance`))))

(event `Key|LeftMouseButton`
  (params (Key :type "Key Structure"))
  (bind _physicshandle (`self.PhysicsHandle`))
  ;[1 1 1] Left click to throw the object
  (:`Pressed`
    (`/Engine/EditorBlueprintResources/StandardMacros.IsValid` _physicshandle
      (:`Is Valid`
        (`PhysicsHandleComponent.ReleaseComponent` _physicshandle)
        (bind (_bblockinghit _binitialoverlap _time _distance _location _impactpoint _normal _impactnormal _physmat _hitactor _hitcomponent _hitbonename) (`GameplayStatics.BreakHitResult` (stale `Key|RightMouseButton` _outhit)))
        (`PrimitiveComponent.AddImpulse` _hitcomponent (* (`SceneComponent.GetForwardVector` (`self.Capsule`)) 5000.0) "None" true)
        ;[1 1 1] Hit conditions
        (`PrimitiveComponent.SetCollisionResponseToChannel` _hitcomponent "ECC_Pawn" "ECR_Block" :!label _label)))))

(event `Key|RightMouseButton`
  (params (Key :type "Key Structure"))
  (bind _physicshandle (`self.PhysicsHandle`))
  (bind _returnvalue (`SceneComponent.K2_GetComponentLocation` (`self.Capsule`)))
  ;[1 1 1] Sets Physics Handle active or not
  (:`Pressed`
    (set `self.PhysicsHandleActive` true)
    ;[1 1 1] Line trace for Physics object
    (bind (_outhit _returnvalue_2) (`KismetSystemLibrary.LineTraceSingleForObjects` :`Start` _returnvalue :`End` (+ _returnvalue (* (`KismetMathLibrary.GetForwardVector` (`self.K2_GetActorRotation` (`GameplayStatics.GetPlayerCameraManager` 0))) (`self.PickUpDistance`))) :`ObjectTypes` (`|MakeArray` (`self.PhysicsObjectType`)) :`DrawDebugType` "ForDuration"))
    (bind (_bblockinghit _binitialoverlap _time _distance _location _impactpoint _normal _impactnormal _physmat _hitactor _hitcomponent _hitbonename) (`GameplayStatics.BreakHitResult` _outhit))
    ;[1 1 1] Get other object location
    (set `self.OtherItemLocation` (`KismetMathLibrary.VSize` (- (`self.K2_GetActorLocation`) _location)))
    (set `self.OtherItemRotation` (`self.K2_GetActorRotation`))
    ;[1 1 1] Hit conditions
    (if _returnvalue_2
      (if (< (`PrimitiveComponent.GetMass` _hitcomponent) 500.0)
        ;[1 1 1] Add grab and physics handle
        (bind _returnvalue_3 (`AddComponent|NODE_AddPhysicsHandleComponent-1`))
        (set `self.PhysicsHandle` _returnvalue_3)
        (set `self.PhysicsObject` _hitcomponent)
        (`PhysicsHandleComponent.GrabComponentAtLocationWithRotation` :`self` (`self.PhysicsHandle`) :`Component` _hitcomponent :`InBoneName` _hitbonename :`Location` _location)
        (`PrimitiveComponent.SetCollisionResponseToChannel` _hitcomponent "ECC_Pawn" "ECR_Ignore"))))
  (:`Released`
    (set `self.PhysicsHandleActive` false)
    (`/Engine/EditorBlueprintResources/StandardMacros.IsValid` _physicshandle
      (:`Is Valid`
        (`PhysicsHandleComponent.ReleaseComponent` _physicshandle)
        (goto _label)))))

(fn `UserConstructionScript`)